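; Player controller that teleports the player pawn to a tagged Transition_BP actor.
; On BeginPlay it sets game-only input and caches all Transition_BP actors in the level.
; The OnTriggerTransition event loops over that cache, checks each actor with GetActorByTag using the hardcoded tag "1", and moves the pawn to the first match's location without sweeping.
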(event Custom|OnTriggerTransition
  (bind _array_element (Utilities|Array|ForEachLoopwithBreak (Variables|Default|GetTransitionActors) :!label _label)
    (:LoopBody
      (bind _res (CallFunction|GetActorbyTag _array_element "1"))
      (if _res
        (Transformation|SetActorLocation (Game|Player|GetPlayerPawn 0) (Transformation|GetActorLocation _array_element) false true)
        (goto _label Break)))))

(event EventBeginPlay
  (Input|SetInputModeGameOnly self)
  (bind _outactors (Actor|GetAllActorsOfClass "/Game/Blueprints/Transition_BP.Transition_BP_C"))
  (Variables|Default|SetTransitionActors _outactors))

(event EventTick
  (params (DeltaSeconds :type Float%20%28single-precision%29)))

(fn ConstructionScript)