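; Third-person player character in a PUBG style, with movement, jump, crouch, sprint, Alt free look, punches, and M16 pickup, holster and aiming.
; A sphere trace finds the rifle, which moves between mesh sockets in step with montages, while flags on PUBG_Anim drive animation states.
; Timelines ease camera arm, FOV, walk speed and free-look return.
; Tick toggles orient-to-movement so the idle camera can see the character's front.
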(event Custom|EquipRifle
  (bind _alpha (Timeline|Attach ReverseFromEnd)
    (:Update
      (Transformation|SetActorTransform (Variables|Default|GetM16) (Math|Transform|Lerp(Transform) (Transformation|GetSocketTransform (Variables|Character|GetMesh) "M16UnEquip" "RTS_World") (Transformation|GetSocketTransform (Variables|Character|GetMesh) "M16" "RTS_World") _alpha)))))

(event Custom|UnEquipRifle
  (bind _alpha (Timeline|Attach PlayFromStart)
    (:Update
      (Transformation|SetActorTransform (Variables|Default|GetM16) (Math|Transform|Lerp(Transform) (Transformation|GetSocketTransform (Variables|Character|GetMesh) "M16UnEquip" "RTS_World") (Transformation|GetSocketTransform (Variables|Character|GetMesh) "M16" "RTS_World") _alpha)))))

(event Custom|StopShooting
  (bind _springarm (Variables|Default|GetSpringArm))
  ;[1 1 1] 瞄准
  (Variables|Default|SetShooting? false)
  (bind (_direction _offset _length) (Timeline|Length Reverse)
    (:Update
      (Variables|/Script/Engine.SpringArmComponent|SetSocketOffset _springarm (Math|Vector|MakeVector (.x (Variables|/Script/Engine.SpringArmComponent|GetSocketOffset _springarm)) _offset (.z (Variables|/Script/Engine.SpringArmComponent|GetSocketOffset _springarm))))
      (Variables|/Script/Engine.SpringArmComponent|SetTargetArmLength _springarm _length))))

(event EventOnLanded
  (params (Hit :type Hit%20Result%20Structure%20%28by%20ref%29))
  (bind _animref (Variables|Default|GetAnimRef))
  ;[1 1 1] 是否着地？
  (Variables|/Game/Blueprints/Player/PUBG_Anim.PUBG_Anim_C|SetOnland _animref true)
  (Utilities|FlowControl|Delay 0.5)
  (Variables|/Game/Blueprints/Player/PUBG_Anim.PUBG_Anim_C|SetOnland _animref false))

(event EventBeginPlay
  ;[1 1 1] 一开始把动画蓝图存为变量，方便后面可以调用
  (bind _aspubg_anim (Utilities|Casting|CastToPUBG_Anim (Components|SkeletalMesh|GetAnimInstance (Variables|Character|GetMesh))))
  (Variables|Default|SetAnimRef _aspubg_anim)
  ;[1 1 1] 当然你们也可以让背包变成可拾取的，然后给角色设置容量，更有可玩性，我这样设置纯粹为了好看!!!!!!!!!
  (bind _returnvalue (Game|SpawnActorfromClass "/Game/Backpack/BackPack.BackPack_C" (Math|Transform|MakeTransform "0, 0, 0") "Undefined" 0 0))
  (bind _output_get (Variables|Default|SetBackPack _returnvalue))
  (Transformation|AttachComponentToComponent _output_get (Variables|Character|GetMesh) "BackPack" "SnapToTarget" "SnapToTarget" "SnapToTarget" true))

(event EventTick
  (params (DeltaSeconds :type Float%20%28single-precision%29))
  ;[1 1 1] 让玩家静止的时候可以看到角色正面
  (if (> (Math|Vector|VectorLength (Transformation|GetVelocity)) 1e+01)
    (if (not (Variables|Default|GetAltPress_))
      (CallFunction|CLoseOrient))
    (else
      ;[1 1 1] 射击的时候角色应该是不能看到正面的
      (if (not (Variables|Default|GetShooting?))
        (CallFunction|OpenOrient)))))

(event Input|ActionEvents|InputActionJump
  (params (Key :type Key%20Structure))
  (bind _animref (Variables|Default|GetAnimRef))
  ;[1 1 1] 跳跃
  (:Pressed
    (if (Variables|Default|GetCanJump_0)
      (Variables|Default|SetCanJump_0 false)
      (Variables|/Game/Blueprints/Player/PUBG_Anim.PUBG_Anim_C|SetJump _animref true)
      (Character|Jump)
      (Utilities|FlowControl|Delay 0.1)
      (Variables|/Game/Blueprints/Player/PUBG_Anim.PUBG_Anim_C|SetJump _animref false)
      (Utilities|FlowControl|Delay 2.0)
      (Variables|Default|SetCanJump_0 true))))

(event Input|AxisEvents|InputAxisMoveForward
  (params (AxisValue :type Float%20%28single-precision%29))
  ;[1 1 1] 玩家移动控制
  (bind _output_get (Variables|Default|SetMoveForward AxisValue))
  (if (Variables|Default|GetAltPress)
    (Pawn|Input|AddMovementInput (Math|Vector|GetForwardVector (Variables|Collision|GetCapsuleComponent)) _output_get false)
    (else
      (Pawn|Input|AddMovementInput (Math|Vector|GetForwardVector (Math|Rotator|MakeRotator 0.0 0.0 (.Yaw (Math|Rotator|BreakRotator (Pawn|GetControlRotation :!class /Script/Engine.Pawn))))) _output_get false))))

(event Input|AxisEvents|InputAxisMoveRight
  (params (AxisValue :type Float%20%28single-precision%29))
  ;[1 1 1] 玩家移动控制
  (bind _output_get (Variables|Default|SetMoveRight AxisValue))
  (Pawn|Input|AddMovementInput (Math|Vector|GetRightVector (Math|Rotator|MakeRotator 0.0 0.0 (.Yaw (Math|Rotator|BreakRotator (Pawn|GetControlRotation :!class /Script/Engine.Pawn))))) _output_get false))

(event Input|AxisEvents|InputAxisLookUp
  (params (AxisValue :type Float%20%28single-precision%29))
  ;[1 1 1] 鼠标控制（我们这里就把人物转向删掉了）
  (Pawn|Input|AddControllerPitchInput AxisValue))

(event Input|AxisEvents|InputAxisTurn
  (params (AxisValue :type Float%20%28single-precision%29))
  ;[1 1 1] 鼠标控制（我们这里就把人物转向删掉了）
  (Pawn|Input|AddControllerYawInput AxisValue))

(event Input|MouseEvents|LeftMouseButton
  (params (Key :type Key%20Structure))
  (bind _mesh (Variables|Character|GetMesh))
  (bind _returnvalue (Components|SkeletalMesh|GetAnimInstance _mesh))
  ;[1 1 1] 打拳
  (:Pressed
    (if (Variables|Default|GetCanPunch)
      (Variables|Default|SetCanPunch false)
      (if (AI|Components|NavMovement|IsFalling (Variables|Character|GetCharacterMovement))
        (bind _returnvalue_2 (Animation|Montage|MontagePlay _returnvalue "/Game/MovementAnimsetPro/Flying_Knee_Punch_Combo_Montage.Flying_Knee_Punch_Combo_Montage" 1.0 "MontageLength" 0.0 true))
        (Utilities|FlowControl|Delay _returnvalue_2)
        (Variables|Default|SetCanPunch true)
        (else
          (bind _returnvalue_3 (Animation|Montage|MontagePlay _returnvalue "/Game/MovementAnimsetPro/Punching__1__Montage.Punching__1__Montage" 1.0 "MontageLength" 0.0 true))
          (Utilities|FlowControl|Delay _returnvalue_3)
          (Variables|Default|SetCanPunch true))))))

(event Input|MouseEvents|RightMouseButton
  (params (Key :type Key%20Structure))
  (bind _springarm (Variables|Default|GetSpringArm))
  ;[1 1 1] 瞄准
  (:Pressed
    (if (Variables|Default|GetRifleState?)
      (Variables|Default|SetShooting? true)
      (CallFunction|CLoseOrient)
      (CallFunction|StopRun)
      (bind (_direction _offset _length) (Timeline|Length Play)
        (:Update
          (Variables|/Script/Engine.SpringArmComponent|SetSocketOffset _springarm (Math|Vector|MakeVector (.x (Variables|/Script/Engine.SpringArmComponent|GetSocketOffset _springarm)) _offset (.z (Variables|/Script/Engine.SpringArmComponent|GetSocketOffset _springarm))))
          (Variables|/Script/Engine.SpringArmComponent|SetTargetArmLength _springarm _length)))))
  (:Released
    (if (Variables|Default|GetRun?)
      (CallFunction|StartRun))
    (Variables|Default|SetShooting? false)
    (Timeline|Length Reverse)))

(event Input|KeyboardEvents|F
  (params (Key :type Key%20Structure))
  (bind _camera (Variables|Default|GetCamera))
  (bind _returnvalue (Transformation|GetWorldLocation _camera))
  ;[1 1 1] 武器的拾取
  (:Pressed
    (bind _outhit (Collision|SphereTraceByChannel _returnvalue (+ _returnvalue (* (Math|Vector|GetForwardVector _camera) 3.5e+02)) 8e+01 "TraceTypeQuery3" false 0 "ForDuration"))
    ;;[1 1 1] 把射线检测碰到的M16存为变量方便后面调用
    (bind _asbp_m16 (Utilities|Casting|CastToBP_M16 (.HitActor (Collision|BreakHitResult _outhit))))
    (Variables|Default|SetM16 _asbp_m16)
    (Utilities|FlowControl|Sequence
      (:then_0
        (Utilities|FlowControl|DoOnce false
          (:Completed
            ;;[1 1 1] 拉出动画蓝图引用设置拾取物品的布尔值
            (Variables|/Game/Blueprints/Player/PUBG_Anim.PUBG_Anim_C|SetIsPickUp? (Variables|Default|GetAnimRef) true)
            ;;[1 1 1] 播放拾取物品的动画
            (Animation|Montage|MontagePlay (Components|SkeletalMesh|GetAnimInstance (Variables|Character|GetMesh)) "/Game/MovementAnimsetPro/Animations/InPlace/PickUp_RH_Montage.PickUp_RH_Montage" 1.0 "MontageLength" 0.0 true)
            ;;[1 1 1] 延迟0.5秒关闭，刚好播到弯腰动画
            (Utilities|FlowControl|Delay 0.5)
            (Variables|/Game/Blueprints/Player/PUBG_Anim.PUBG_Anim_C|SetIsPickUp? (Variables|Default|GetAnimRef) false)
            ;;[1 1 1] 把拾取的M16附着到角色身上
            (Transformation|AttachComponentToComponent (Variables|Default|GetM16) (Variables|Character|GetMesh) "M16" "SnapToTarget" "SnapToTarget" "SnapToTarget" true)
            ;;[1 1 1] 同时把M16身上的球形碰撞关闭，防止多次触发拾取
            (Collision|SetCollisionEnabled (Variables|/Game/M16/Blueprint/BP_M16.BP_M16_C|GetSphere (Variables|Default|GetM16)) "NoCollision")
            ;;[1 1 1] 同时创建一个布尔值，判断是否有武器
            (Variables|Default|SetHaveRifle? true)))))))

(event Input|KeyboardEvents|1
  (params (Key :type Key%20Structure))
  ;[1 1 1] 装备武器
  (:Pressed
    (if (Variables|Default|GetHaveRifle?)
      ;;[1 1 1] 是否可以装备武器
      (if (Variables|Default|GetCanEquipRifle)
        (Variables|Default|SetCanEquipRifle false)
        ;;[1 1 1] 当前是否是持枪状态
        (if (Variables|Default|GetRifleState?)
          (Variables|Default|SetRifleState? false)
          (Animation|Montage|MontagePlay (Components|SkeletalMesh|GetAnimInstance (Variables|Character|GetMesh)) "/Game/RifleAnimsetPro/Animations/InPlace/HolsterRifle_Montage.HolsterRifle_Montage" 1.0 "MontageLength" 0.0 true)
          (Utilities|FlowControl|Delay 1.0)
          ;;[1 1 1] 关闭持枪状态
          (Variables|/Game/Blueprints/Player/PUBG_Anim.PUBG_Anim_C|SetRifleState (Variables|Default|GetAnimRef) false)
          (CallFunction|UnEquipRifle)
          (Transformation|AttachComponentToComponent (Variables|Default|GetM16) (Variables|Character|GetMesh) "M16UnEquip" "SnapToTarget" "SnapToTarget" "SnapToTarget" true)
          (Utilities|FlowControl|Delay 2.0)
          ;;[1 1 1] 这个布尔值来混合装备与行走跑步的动画
          (Variables|Default|SetCanEquipRifle true)
          (else
            (Variables|Default|SetRifleState? true)
            (Animation|Montage|MontagePlay (Components|SkeletalMesh|GetAnimInstance (Variables|Character|GetMesh)) "/Game/RifleAnimsetPro/Animations/InPlace/EquipRifle_Montage.EquipRifle_Montage" 1.0 "MontageLength" 0.0 true)
            (Utilities|FlowControl|Sequence
              (:then_0
                (CallFunction|EquipRifle))
              (:then_1
                ;;[1 1 1] 0.47秒刚好到角色掏枪的位置
                (Utilities|FlowControl|Delay 0.47)
                (Transformation|AttachComponentToComponent (Variables|Default|GetM16) (Variables|Character|GetMesh) "M16Equip" "SnapToTarget" "SnapToTarget" "SnapToTarget" true)
                (Utilities|FlowControl|Delay 2.0)
                (Variables|Default|SetCanEquipRifle true))
              (:then_2
                ;;[1 1 1] 开启持枪状态
                (Utilities|FlowControl|Delay 0.5)
                (Variables|/Game/Blueprints/Player/PUBG_Anim.PUBG_Anim_C|SetRifleState (Variables|Default|GetAnimRef) true)))))))))

(event Input|KeyboardEvents|LeftAlt
  (params (Key :type Key%20Structure))
  ;[1 1 1] 简易版自由视角(Bug 多多)
  (:Pressed
    (Utilities|FlowControl|Sequence
      (:then_0
        (Variables|Default|SetAltPress_ true)
        (Variables|Default|SetAltPress true)
        (Variables|Default|SetbUseControllerRotationYaw false))
      (:then_1
        (bind _newtrack_0 (Timeline|AltFreeLook Stop)
          (:Update
            (Pawn|SetControlRotation (Game|GetPlayerController 0) (Math|Rotator|Lerp(Rotator) (Pawn|GetControlRotation :!class /Script/Engine.Pawn) (Transformation|GetWorldRotation (Variables|Collision|GetCapsuleComponent)) _newtrack_0 true)))
          (:Finished
            (Variables|Default|SetbUseControllerRotationYaw true)
            (Variables|Default|SetAltPress_ false))))))
  (:Released
    (Variables|Default|SetAltPress false)
    (Timeline|AltFreeLook PlayFromStart)))

(fn ConstructionScript)

(fn OpenOrient
  (Variables|/Script/Engine.CharacterMovementComponent|SetbOrientRotationToMovement (Variables|Character|GetCharacterMovement) true)
  (Variables|Default|SetbUseControllerRotationYaw false))

(fn CLoseOrient
  (Variables|/Script/Engine.CharacterMovementComponent|SetbOrientRotationToMovement (Variables|Character|GetCharacterMovement) false)
  (Variables|Default|SetbUseControllerRotationYaw true))

(event Input|KeyboardEvents|C
  (params (Key :type Key%20Structure))
  (bind _springarm (Variables|Default|GetSpringArm))
  ;[1 1 1] Crouch
  (:Pressed
    (if (Variables|Default|GetCanCrouch)
      (Variables|Default|SetCanCrouch false)
      (Utilities|FlowControl|FlipFlop
        (:A
          (Character|Crouch)
          (bind _newtrack_0 (Timeline|Crouch PlayFromStart)
            (:Update
              (Variables|/Script/Engine.SpringArmComponent|SetSocketOffset _springarm (Math|Vector|MakeVector 0.0 (.y (Variables|/Script/Engine.SpringArmComponent|GetSocketOffset _springarm)) _newtrack_0)))
            (:Finished
              (Utilities|FlowControl|Delay 0.5)
              (Variables|Default|SetCanCrouch true))))
        (:B
          (Character|UnCrouch)
          (Timeline|Crouch ReverseFromEnd))))))

(event Custom|StartRun
  ;[1 1 1] Run
  (bind (_direction _run _field) (Timeline|Run Play)
    (:Update
      (Variables|/Script/Engine.CharacterMovementComponent|SetMaxWalkSpeed (Variables|Character|GetCharacterMovement) _run)
      (Camera|SetFieldOfView (Variables|Default|GetCamera) _field))))

(event Custom|StopRun
  ;[1 1 1] Run
  (bind (_direction _run _field) (Timeline|Run Reverse)
    (:Update
      (Variables|/Script/Engine.CharacterMovementComponent|SetMaxWalkSpeed (Variables|Character|GetCharacterMovement) _run)
      (Camera|SetFieldOfView (Variables|Default|GetCamera) _field))))

(event Input|ActionEvents|InputActionRun
  (params (Key :type Key%20Structure))
  ;[1 1 1] Run
  (:Pressed
    (if (not (AI|Components|NavMovement|IsCrouching (Variables|Character|GetCharacterMovement)))
      (CallFunction|StopShooting)
      (Variables|Default|SetRun? true)
      (bind (_direction _run _field) (Timeline|Run Play)
        (:Update
          (Variables|/Script/Engine.CharacterMovementComponent|SetMaxWalkSpeed (Variables|Character|GetCharacterMovement) _run)
          (Camera|SetFieldOfView (Variables|Default|GetCamera) _field)))))
  (:Released
    (Utilities|FlowControl|Sequence
      (:then_0
        (Timeline|Run Reverse))
      (:then_1
        (Utilities|FlowControl|Delay 0.2)
        (Variables|Default|SetRun? false)))))